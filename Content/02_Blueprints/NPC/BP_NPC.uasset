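; Clickable NPC character that toggles a dialogue view in a top-down game.
; A sphere overlap tracks player range, gating capsule clicks that show or hide a widget and blend the camera between NPC and player.
; Cursor hover applies an overlay material, and Tick rotates the widget toward the camera's relative location.
; UI hide/show logic never runs; a Dash function launches the NPC forward.
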(event `Enter_Dialogue`
  (`SceneComponent.SetVisibility` (`self.Widget`) true false)
  (`PlayerController.SetViewTargetWithBlend` (`/Game/02_Blueprints/BP_FL_Getters.GetTopDownPlayerController`) self 1.0 "VTBlend_Linear" 0.0 false))

(event `Quit_Dialogue`
  (`SceneComponent.SetVisibility` (`self.Widget`) false false)
  (`PlayerController.SetViewTargetWithBlend` (`/Game/02_Blueprints/BP_FL_Getters.GetTopDownPlayerController`) (`/Game/02_Blueprints/BP_FL_Getters.GetTopDownPlayerCharacter`) 0.5 "VTBlend_Linear" 0.0 false))

(event `self.ReceiveTick`
  (params (DeltaSeconds :type "Float (single-precision)"))
  (`SceneComponent.K2_SetWorldRotation` (`self.Widget`) (`KismetMathLibrary.FindLookAtRotation` (`SceneComponent.K2_GetComponentLocation` (`self.Widget`)) (`SceneComponent.RelativeLocation` (`self.Camera`))) false false))

(event `self.CapsuleComponent.OnBeginCursorOver`
  (params (TouchedComponent :type "PrimitiveComponent Object Reference"))
  (`MeshComponent.SetOverlayMaterial` (`self.Mesh`) "/Game/04_Materials/M_InractionNPCOverlay.M_InractionNPCOverlay"))

(event `self.CapsuleComponent.OnEndCursorOver`
  (params (TouchedComponent :type "PrimitiveComponent Object Reference"))
  (`MeshComponent.SetOverlayMaterial` (`self.Mesh`) null))

(event `self.CapsuleComponent.OnClicked`
  (params (TouchedComponent :type "PrimitiveComponent Object Reference") (ButtonPressed :type "Key Structure"))
  (if (`self.Player_Is_In_Range`)
    (if (`self.Is_In_Dialogue`)
      (`self.Quit_Dialogue`)
      (set `self.Is_In_Dialogue` false)
      (else
        (`self.Enter_Dialogue`)
        (set `self.Is_In_Dialogue` true)
        (`MeshComponent.SetOverlayMaterial` (`self.Mesh`) null)))
    (else
      (`KismetSystemLibrary.PrintString` "not in range")
      (`/Game/02_Blueprints/BP_TopDownCharacter.Character_Movement` (`/Game/02_Blueprints/BP_FL_Getters.GetTopDownPlayerCharacter`) 30.0))))

(event `self.Sphere.OnComponentBeginOverlap`
  (params (OverlappedComponent :type "PrimitiveComponent Object Reference") (OtherActor :type "Actor Object Reference") (OtherComp :type "PrimitiveComponent Object Reference") (OtherBodyIndex :type Integer) (bFromSweep :type Boolean) (SweepResult :type "HitResult Structure (by ref)"))
  (if (== OtherActor (`/Game/02_Blueprints/BP_FL_Getters.GetTopDownPlayerCharacter`))
    (set `self.Player_Is_In_Range` true)))

(event `self.Sphere.OnComponentEndOverlap`
  (params (OverlappedComponent :type "PrimitiveComponent Object Reference") (OtherActor :type "Actor Object Reference") (OtherComp :type "PrimitiveComponent Object Reference") (OtherBodyIndex :type Integer))
  (if (== OtherActor (`/Game/02_Blueprints/BP_FL_Getters.GetTopDownPlayerCharacter`))
    (set `self.Player_Is_In_Range` false)))

(fn `Dash`
  (`self.LaunchCharacter` (* (`self.GetActorForwardVector` self) 5.0) true true))

(fn `UserConstructionScript`)