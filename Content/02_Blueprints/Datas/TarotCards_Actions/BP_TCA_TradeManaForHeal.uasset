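; Tarot card action that changes the player's mana and life, named as a trade of mana for healing.
; LaunchConverted stores the passed controller, then adds ManaChange to its current mana and HealChange to its current life.
; Each result is capped only at its maximum, with no lower clamp.
; The matching player UI bar then updates using the value divided by a fixed 100 rather than the maximum.
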(fn `LaunchConverted`
  (params (Controller :type "/Game/02_Blueprints/BP_TopDownController Object Reference"))
  (locals (`Controller Ref` :type "/Game/02_Blueprints/BP_TopDownController Object Reference"))
  (bind _controller_ref (`local.Controller Ref`))
  (bind _controller_ref_2 (`local.Controller Ref`))
  (bind _controller_ref_3 (`local.Controller Ref`))
  (bind _controller_ref_4 (`local.Controller Ref`))
  (set `local.Controller Ref` Controller)
  (`|ExecutionSequence`
    (:`then_0`
      (bind _output_get (set `/Game/02_Blueprints/BP_TopDownController.Current_Mana` (+ (`/Game/02_Blueprints/BP_TopDownController.Current_Mana` (`local.Controller Ref`)) (`self.Mana_Change`)) _controller_ref_4))
      (if (>= _output_get (`/Game/02_Blueprints/BP_TopDownController.Max_Mana` _controller_ref_4))
        (bind _output_get_2 (set `/Game/02_Blueprints/BP_TopDownController.Current_Mana` (`/Game/02_Blueprints/BP_TopDownController.Max_Mana` _controller_ref_2) _controller_ref_2))
        (`/Game/02_Blueprints/UI/WBP_PlayerUI.Update_ManaBar` (`/Game/02_Blueprints/BP_TopDownController.Player_UI` (`local.Controller Ref`)) (/ _output_get_2 100.0))
        (else
          (`/Game/02_Blueprints/UI/WBP_PlayerUI.Update_ManaBar` (`/Game/02_Blueprints/BP_TopDownController.Player_UI` (`local.Controller Ref`)) (/ (`/Game/02_Blueprints/BP_TopDownController.Current_Mana` (`local.Controller Ref`)) 100.0)))))
    (:`then_1`
      (bind _output_get_3 (set `/Game/02_Blueprints/BP_TopDownController.Current_Life` (+ (`/Game/02_Blueprints/BP_TopDownController.Current_Life` (`local.Controller Ref`)) (`self.Heal_Change`)) _controller_ref))
      (if (>= _output_get_3 (`/Game/02_Blueprints/BP_TopDownController.Max_Life` _controller_ref))
        (bind _output_get_4 (set `/Game/02_Blueprints/BP_TopDownController.Current_Life` (`/Game/02_Blueprints/BP_TopDownController.Max_Life` _controller_ref_3) _controller_ref_3))
        (`/Game/02_Blueprints/UI/WBP_PlayerUI.Update_LifeBar` (`/Game/02_Blueprints/BP_TopDownController.Player_UI` (`local.Controller Ref`)) (/ _output_get_4 100.0))
        (else
          (`/Game/02_Blueprints/UI/WBP_PlayerUI.Update_LifeBar` (`/Game/02_Blueprints/BP_TopDownController.Player_UI` (`local.Controller Ref`)) (/ (`/Game/02_Blueprints/BP_TopDownController.Current_Life` (`local.Controller Ref`)) 100.0)))))))