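; Tarot card action that changes the controller's mana, named for mana recovery.
; LaunchConverted adds ManaChange to CurrentMana and caps the result at MaxMana, with no lower clamp.
; It then refreshes the player UI with CurrentMana divided by a fixed 100 rather than by MaxMana.
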(fn `LaunchConverted`
  (params (Controller :type "/Game/02_Blueprints/BP_TopDownController Object Reference"))
  (bind _max_mana (`/Game/02_Blueprints/BP_TopDownController.Max_Mana` Controller))
  (bind _output_get (set `/Game/02_Blueprints/BP_TopDownController.Current_Mana` (+ (`/Game/02_Blueprints/BP_TopDownController.Current_Mana` Controller) (`self.Mana_Change`)) Controller))
  (if (>= _output_get _max_mana)
    (bind _output_get_2 (set `/Game/02_Blueprints/BP_TopDownController.Current_Mana` _max_mana Controller)))
  (`/Game/02_Blueprints/UI/WBP_PlayerUI.Update_Mana` (`/Game/02_Blueprints/BP_TopDownController.Player_UI` Controller) (/ _output_get_2 100.0)))