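; BP_NPC is an NPC actor that offers a dialogue view to the player in a top-down game.
; Any overlap on its Sphere sets or clears it as CurrentNPC on BP_TopDownController, without checking the overlapping actor.
; Dialogue shows the Widget and blends the player's view to the NPC, while Hide only hides the Widget.
; Tick rotates the Widget using the Camera's forward vector as the look-at target, rather than its location.
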(event `Hide`
  (`SceneComponent.SetVisibility` (`self.Widget`) false false))

(event `Dialogue`
  (`SceneComponent.SetVisibility` (`self.Widget`) true false)
  (`PlayerController.SetViewTargetWithBlend` (`GameplayStatics.GetPlayerController` 0) self 1.0 "VTBlend_Linear" 0.0 false))

(event `self.ReceiveTick`
  (params (DeltaSeconds :type "Float (single-precision)"))
  (bind _widget (`self.Widget`))
  (`SceneComponent.K2_SetWorldRotation` _widget (`KismetMathLibrary.FindLookAtRotation` (`SceneComponent.K2_GetComponentLocation` _widget) (`SceneComponent.GetForwardVector` (`self.Camera`))) false false))

(event `self.Sphere.OnComponentBeginOverlap`
  (params (OverlappedComponent :type "PrimitiveComponent Object Reference") (OtherActor :type "Actor Object Reference") (OtherComp :type "PrimitiveComponent Object Reference") (OtherBodyIndex :type Integer) (bFromSweep :type Boolean) (SweepResult :type "HitResult Structure (by ref)"))
  (bind _asbp_top_down_controller (cast `/Game/TopDown/Blueprints/BP_TopDownController` (`GameplayStatics.GetPlayerController` 0)))
  (set `/Game/TopDown/Blueprints/BP_TopDownController.CurrentNPC` self _asbp_top_down_controller))

(event `self.Sphere.OnComponentEndOverlap`
  (params (OverlappedComponent :type "PrimitiveComponent Object Reference") (OtherActor :type "Actor Object Reference") (OtherComp :type "PrimitiveComponent Object Reference") (OtherBodyIndex :type Integer))
  (bind _asbp_top_down_controller (cast `/Game/TopDown/Blueprints/BP_TopDownController` (`GameplayStatics.GetPlayerController` 0)))
  (set `/Game/TopDown/Blueprints/BP_TopDownController.CurrentNPC` null _asbp_top_down_controller))

(fn `UserConstructionScript`)