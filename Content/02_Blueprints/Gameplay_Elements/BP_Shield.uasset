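; BP_Shield is a shield actor that attaches to the top-down player character on spawn.
; On BeginPlay it snaps to the player's location, keeping relative rotation and world scale, then starts a self-destruct.
; The self-destruct waits for the cooldown from the shield data asset and destroys the actor.
; An unused timeline that prints its track value is left disconnected.
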(event `self.ReceiveBeginPlay`
  (`self.K2_AttachToActor` (`/Game/02_Blueprints/BP_FL_Getters.GetTopDownPlayerCharacter`) "None" "SnapToTarget" "KeepRelative" "KeepWorld")
  (`self.Self_Destruct`))

(event `Self_Destruct`
  (`KismetSystemLibrary.Delay` (`/Game/02_Blueprints/Datas/BP_DA_Spell.CoolDown` (`self.DA_Shield`)))
  (`self.K2_DestroyActor`))

(fn `UserConstructionScript`)