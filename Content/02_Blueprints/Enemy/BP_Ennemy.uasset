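; BP_Ennemy is an enemy whose AI reacts to the player's proximity through Blackboard flags.
; On BeginPlay it applies the MI_Ennemy overlay material to its mesh.
; When the player character enters or leaves its Sphere, it toggles PlayerIsInRange and CanMove inversely on its AI controller's Blackboard, so CanMove is false while the player is in range.
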(event `self.ReceiveBeginPlay`
  (`MeshComponent.SetOverlayMaterial` (`self.Mesh`) "/Game/04_Materials/Animated_Materials/MI_Ennemy.MI_Ennemy"))

(event `self.Sphere.OnComponentBeginOverlap`
  (params (OverlappedComponent :type "PrimitiveComponent Object Reference") (OtherActor :type "Actor Object Reference") (OtherComp :type "PrimitiveComponent Object Reference") (OtherBodyIndex :type Integer) (bFromSweep :type Boolean) (SweepResult :type "HitResult Structure (by ref)"))
  (if (== OtherActor (`/Game/02_Blueprints/BP_FL_Getters.Get_Player_Character`))
    (`BlackboardComponent.SetValueAsBool` (`AIBlueprintHelperLibrary.GetBlackboard` (`AIBlueprintHelperLibrary.GetAIController` self)) (`self.Player_Is_In_Range`) true)
    (`BlackboardComponent.SetValueAsBool` (`AIBlueprintHelperLibrary.GetBlackboard` (`AIBlueprintHelperLibrary.GetAIController` self)) (`self.Can_Move`) false)))

(event `self.Sphere.OnComponentEndOverlap`
  (params (OverlappedComponent :type "PrimitiveComponent Object Reference") (OtherActor :type "Actor Object Reference") (OtherComp :type "PrimitiveComponent Object Reference") (OtherBodyIndex :type Integer))
  (if (== OtherActor (`/Game/02_Blueprints/BP_FL_Getters.Get_Player_Character`))
    (`BlackboardComponent.SetValueAsBool` (`AIBlueprintHelperLibrary.GetBlackboard` (`AIBlueprintHelperLibrary.GetAIController` self)) (`self.Player_Is_In_Range`) false)
    (`BlackboardComponent.SetValueAsBool` (`AIBlueprintHelperLibrary.GetBlackboard` (`AIBlueprintHelperLibrary.GetAIController` self)) (`self.Can_Move`) true)))

(fn `UserConstructionScript`)